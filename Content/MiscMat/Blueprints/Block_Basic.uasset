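; Block_Basic is a block actor that can be picked up and dropped, showing its state by swapping its material's base color texture.
; Focus shows one texture, while pickup/drop and physics wake/sleep events set flags that ChangeTextureByState maps to free-moving, free-sleeping or held textures.
; Tick spins the block on flagged axes, and RestoreRotation resets it.
; Face attachment is a TODO stub, EnablePhysics is never reached from the event graph, and LaunchRayLength traces from the camera.
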(event OnComponentWake(StaticMeshComponent)
  (params (WakingComponent :type Primitive%20Component%20Object%20Reference) (BoneName :type Name :default "None"))
  ;[1 1 1] Rigid Body Events
  (Variables|Default|SetIsSleeping false)
  (CallFunction|ChangeTexturebyState))

(event OnComponentSleep(StaticMeshComponent)
  (params (SleepingComponent :type Primitive%20Component%20Object%20Reference) (BoneName :type Name :default "None"))
  ;[1 1 1] Rigid Body Events
  (Variables|Default|SetIsSleeping true)
  (CallFunction|ChangeTexturebyState))

(event Custom|ChangeTextureByState
  (bind _blockmaterial (Variables|Default|GetBlockMaterial))
  ;[1 1 1] Change Texture By State
  (if (Variables|Default|GetIsFree)
    (if (Variables|Default|GetIsSleeping)
      (Rendering|Material|SetTextureParameterValue _blockmaterial "TexBaseColor" "/Game/Textures/T_FaceB.T_FaceB")
      (else
        (Rendering|Material|SetTextureParameterValue _blockmaterial "TexBaseColor" "/Game/Textures/T_FaceA.T_FaceA")))
    (else
      (Rendering|Material|SetTextureParameterValue (Variables|Default|GetBlockMaterial) "TexBaseColor" "/Game/Textures/T_FaceD.T_FaceD"))))

(event Custom|AttachToFace
  ;[1 1 1] TODO: LineTrace from each side of the block to detect other faces; then free the block and set its location
  (Utilities|Array|Add (Variables|Default|GetNewVar_0) self))

(event Custom|RestoreRotation
  (Transformation|SetActorRotation "0, 0, 0"))

(event Custom|On%20Pickup
  ;[1 1 1] Pickup & Drop
  (Variables|Default|SetIsFree false)
  (CallFunction|ChangeTexturebyState))

(event Custom|On%20Drop
  ;[1 1 1] Pickup & Drop
  (Variables|Default|SetIsFree true)
  (CallFunction|ChangeTexturebyState))

(event Custom|On%20Focus
  ;[1 1 1] Focus Change Events
  (Rendering|Material|SetTextureParameterValue (Variables|Default|GetBlockMaterial) "TexBaseColor" "/Game/Textures/T_FaceC.T_FaceC"))

(event Custom|Lost%20Focus
  ;[1 1 1] Focus Change Events
  (CallFunction|ChangeTexturebyState))

(event EventTick
  (params (DeltaSeconds :type Float%20%28single-precision%29))
  (Utilities|FlowControl|Sequence
    (:then_0
      (if (Variables|Default|GetRotateX)
        (Class|Actor|AddActorWorldRotation "0, 0,1.000000")))
    (:then_1
      (if (Variables|Default|GetRotateY)
        (Class|Actor|AddActorWorldRotation "1.000000, 0,0.000000")))
    (:then_2
      (if (Variables|Default|GetRotateZ)
        (Class|Actor|AddActorWorldRotation "0,1.000000, 0")))))

(fn ConstructionScript
  (Rendering|Material|SetMaterial (Variables|Default|GetCube) 0 "/Game/Materials/M_Bloks.M_Bloks"))

(fn EnablePhysics
  (params (Bool :type Boolean))
  (bind _cube (Variables|Default|GetCube))
  (Collision|SetCollisionEnabled _cube "QueryAndPhysics")
  (Physics|SetSimulatePhysics _cube Bool)
  (if Bool
    (Collision|SetCollisionEnabled _cube "QueryAndPhysics")
    (else
      (Collision|SetCollisionEnabled _cube "NoCollision"))))